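; HUD actor for the boat game that owns the gameplay and game-over screens.
; On BeginPlay it creates and displays WBP_GamePlayHud, then hands that widget reference to the player's BP_BoatPawn.
; Its GameOver event removes the gameplay widget and shows WBP_GameOver, with the passed integer displayed as the score.
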(event `self.ReceiveBeginPlay`
  (bind _returnvalue (`|CreateWidget` "/Game/BluePrint/WBP_GamePlayHud.WBP_GamePlayHud_C" (`GameplayStatics.GetPlayerController` 0)))
  (bind _output_get (set `self.MainWidget` _returnvalue))
  (`UserWidget.AddToViewport` _output_get 0)
  (bind _asbp_boat_pawn (cast `/Game/BluePrint/BP_BoatPawn` (`GameplayStatics.GetPlayerPawn` 0)))
  (set `BoatPawn.MainWidget` _output_get _asbp_boat_pawn))

(event `GameOver`
  (params (NewParam :type Integer))
  (`Widget.RemoveFromParent` (`self.MainWidget`))
  (bind _returnvalue (`|CreateWidget` "/Game/UI/WBP_GameOver.WBP_GameOver_C" (`GameplayStatics.GetPlayerController` 0)))
  (set `TextBlock.Text` (`KismetTextLibrary.Conv_IntToText` NewParam) (`/Game/UI/WBP_GameOver.Score` _returnvalue))
  (`UserWidget.AddToViewport` _returnvalue 0))

(fn `UserConstructionScript`)