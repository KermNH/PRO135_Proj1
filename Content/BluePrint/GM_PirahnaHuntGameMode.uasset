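; GM_PirahnaHuntGameMode is the game mode for Piranha Hunt, handling match start and game over.
; On BeginPlay it shows the mouse cursor, sets game-and-UI input mode locked on capture, and starts the music.
; Its GameOver event pauses the game and passes the Score to the HUD_MainHud's GameOver.
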(event `self.ReceiveBeginPlay`
  (bind _returnvalue (`GameplayStatics.GetPlayerController` 0))
  (`|ExecutionSequence`
    (:`then_0`
      (set `PlayerController.bShowMouseCursor` true _returnvalue)
      (`WidgetBlueprintLibrary.SetInputMode_GameAndUIEx` _returnvalue null "LockOnCapture" false))
    (:`then_1`
      (`GameplayStatics.PlaySound2D` "/Game/Assets/SFX/SC_Music.SC_Music" 1.0 1.0 0.0 null null))))

(event `self.GameOver`
  (`GameplayStatics.SetGamePaused` true)
  (bind _ashud_main_hud (cast `/Game/BluePrint/HUD_MainHud` (`PlayerController.GetHUD` (`GameplayStatics.GetPlayerController` 0))))
  (`/Game/BluePrint/HUD_MainHud.GameOver` _ashud_main_hud (`self.Score`)))

(fn `UserConstructionScript`)